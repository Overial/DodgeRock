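; Player controller for the DodgeRock game that owns input handling and the pause menu.
; On BeginPlay it sets game-only input, adds the Enhanced Input mapping context and caches the possessed character's movement component.
; Move input feeds control-rotation-relative vectors straight into that component, while look input drives yaw and pitch.
; The pause action toggles game pause, showing or removing a lazily created, reused menu widget and switching input mode and cursor.
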(event Input|EnhancedActionEvents|EnhancedInputActionIA_DodgeRockMove
  (params (ActionValue :type Vector%202D%20Structure) (ElapsedSeconds :type Float%20%28double-precision%29) (TriggeredSeconds :type Float%20%28double-precision%29) (InputAction :type Input%20Action%20Object%20Reference :default "/Game/DodgeRock/Core/EnhancedInput/Action/IA_DodgeRockMove.IA_DodgeRockMove"))
  (bind _returnvalue (Pawn|GetControlRotation :!class /Script/Engine.Controller))
  (:Triggered
    (bind _charactermovementcomp (Variables|Default|GetCharacterMovementComp)
      (:then
        (Utilities|FlowControl|Sequence
          (:then_0
            (Class|PawnMovementComponent|AddInputVector _charactermovementcomp (* (Math|Vector|GetForwardVector (Math|Rotator|MakeRotator 0.0 0.0 (.yaw (Pawn|GetControlRotation :!class /Script/Engine.Controller)))) (.y ActionValue)) false))
          (:then_1
            (Class|PawnMovementComponent|AddInputVector _charactermovementcomp (* (Math|Vector|GetRightVector (Math|Rotator|MakeRotator (.roll _returnvalue) 0.0 (.yaw _returnvalue))) (.x ActionValue)) false))))
      (:else))))

(event Input|EnhancedActionEvents|EnhancedInputActionIA_DodgeRockLook
  (params (ActionValue :type Vector%202D%20Structure) (ElapsedSeconds :type Float%20%28double-precision%29) (TriggeredSeconds :type Float%20%28double-precision%29) (InputAction :type Input%20Action%20Object%20Reference :default "/Game/DodgeRock/Core/EnhancedInput/Action/IA_DodgeRockLook.IA_DodgeRockLook"))
  (:Triggered
    (Class|PlayerController|AddYawInput (.x ActionValue))
    (Class|PlayerController|AddPitchInput (.y ActionValue))))

(event Input|EnhancedActionEvents|EnhancedInputActionIA_DodgeRockPauseMenu
  (params (ActionValue :type Boolean) (ElapsedSeconds :type Float%20%28double-precision%29) (TriggeredSeconds :type Float%20%28double-precision%29) (InputAction :type Input%20Action%20Object%20Reference :default "/Game/DodgeRock/Core/EnhancedInput/Action/IA_DodgeRockPauseMenu.IA_DodgeRockPauseMenu"))
  (:Triggered
    (if (Game|IsGamePaused)
      (Game|SetGamePaused false)
      (Input|SetInputModeGameOnly self false)
      (Variables|Default|SetbShowMouseCursor false)
      (bind _pausemenuwidget (Variables|Default|GetPauseMenuWidget)
        (:then
          (Widget|RemovefromParent _pausemenuwidget))
        (:else))
      (else
        (Game|SetGamePaused true)
        (Variables|Default|GetPauseMenuWidget
          (:then
            _)
          (:else
            (bind _returnvalue (UserInterface|CreateWidget "/Game/DodgeRock/UI/WBP_PauseMenu.WBP_PauseMenu_C" self))
            (bind _output_get (Variables|Default|SetPauseMenuWidget _returnvalue))))
        (UserInterface|Viewport|AddtoViewport _output_get 0)
        (Input|SetInputModeGameandUI self _output_get "DoNotLock" true false)
        (Variables|Default|SetbShowMouseCursor true)))))

(event EventBeginPlay
  (bind _self self)
  (Input|SetInputModeGameOnly _self false)
  (Variables|Default|SetbShowMouseCursor _self false)
  (Input|AddMappingContext (PlayerController|LocalPlayerSubsystems|GetEnhancedInputLocalPlayerSubsystem) "/Game/DodgeRock/Core/EnhancedInput/IMC_DodgeRock.IMC_DodgeRock" 0 "(bIgnoreAllPressedKeysUntilRelease=True,bForceImmediately=False)")
  (bind _asbp_dodge_rock_character (Utilities|Casting|CastToBP_DodgeRockCharacter (Pawn|GetControlledPawn)))
  (bind _output_get (Variables|Default|SetDodgeRockCharacter _asbp_dodge_rock_character))
  (Variables|Default|SetCharacterMovementComp (Variables|/Script/Engine.Character|GetCharacterMovement _output_get)))

(fn ConstructionScript)