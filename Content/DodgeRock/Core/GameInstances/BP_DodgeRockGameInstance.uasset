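; Game instance for DodgeRock that holds the selected game difficulty and the highest score.
; Getter and setter functions wrap both values.
; The high score setter only overwrites the stored value when the new score is greater, while difficulty is assigned directly.
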(fn SetGameDifficulty
  (params (GameDifficulty :type EGameDifficulty%20Enum :default "NewEnumerator0"))
  (Variables|Default|SetGameDifficulty GameDifficulty))

(fn GetGameDifficulty
  (return (Variables|Default|GetGameDifficulty)))

(fn SetHighestScore
  (params (HighestScore :type Integer))
  (if (> HighestScore (CallFunction|GetHighestScore))
    (Variables|Default|SetHighestScore HighestScore)))

(fn GetHighestScore
  (return (Variables|Default|GetHighestScore)))